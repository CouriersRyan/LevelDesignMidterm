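; Package is a collectible delivery pickup that spins and bobs in place using yaw rotation and a sine-wave height offset on Tick.
; On BeginPlay it adds itself to the first-person character's TotalPackages count.
; When that character overlaps its Box, it increments PackagesPickedUp, plays a sound, calls Delivery on its assigned DeliveryDropOff and destroys itself.
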(event OnComponentBeginOverlap(Box)
  (params (OverlappedComponent :type Primitive%20Component%20Object%20Reference) (OtherActor :type Actor%20Object%20Reference) (OtherComp :type Primitive%20Component%20Object%20Reference) (OtherBodyIndex :type Integer) (bFromSweep :type Boolean) (SweepResult :type Hit%20Result%20Structure%20%28by%20ref%29))
  (bind _asbp_first_person_character (Utilities|Casting|CastToBP_FirstPersonCharacter OtherActor))
  (Math|Integer|IncrementInt (Variables|/Game/FirstPerson/Blueprints/BP_FirstPersonCharacter.BP_FirstPersonCharacter_C|GetPackages%20Picked%20Up _asbp_first_person_character)
    (:%20%20
      (Audio|PlaySound2D "/Engine/VREditor/Sounds/UI/Camera_Shutter.Camera_Shutter" 1.0 1.0 0.0 0 0)
      (bind _asdelivery_drop_off (Utilities|Casting|CastToDeliveryDropOff (Variables|Default|GetDelivery%20Location)))
      (Default|Delivery _asdelivery_drop_off)
      (Actor|DestroyActor))))

(event EventBeginPlay
  (Variables|Default|SetStarting%20Location (Variables|/Script/Engine.SceneComponent|GetRelativeLocation (Variables|Default|GetPackage)))
  (bind _asbp_first_person_character (Utilities|Casting|CastToBP_FirstPersonCharacter (Game|GetPlayerCharacter 0)))
  (Math|Integer|IncrementInt (Variables|/Game/FirstPerson/Blueprints/BP_FirstPersonCharacter.BP_FirstPersonCharacter_C|GetTotal%20Packages _asbp_first_person_character)))

(event EventTick
  (params (DeltaSeconds :type Float%20%28single-precision%29))
  (bind _package (Variables|Default|GetPackage))
  (Transformation|AddLocalRotation _package (Math|Rotator|MakeRotator 0.0 0.0 (* DeltaSeconds 25.0)) false false)
  (Transformation|SetRelativeLocation _package (+ (Variables|Default|GetStarting%20Location) (Math|Vector|MakeVector 0.0 0.0 (* (Math|Trig|Sin(Radians) (Utilities|Time|GetTimeSeconds)) 16.0))) true false))

(fn ConstructionScript)