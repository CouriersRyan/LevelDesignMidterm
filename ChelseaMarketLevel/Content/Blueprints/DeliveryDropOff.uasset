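; DeliveryDropOff is a drop-off point where the first-person character completes pending deliveries.
; Its Delivery event increments a pending count, flags that a delivery exists and shows the Waypoint component.
; When the character overlaps the Box while deliveries are pending, it passes the count to the character's DropOff, then resets the count and flag and hides the waypoint.
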(event OnComponentBeginOverlap(Box)
  (params (OverlappedComponent :type Primitive%20Component%20Object%20Reference) (OtherActor :type Actor%20Object%20Reference) (OtherComp :type Primitive%20Component%20Object%20Reference) (OtherBodyIndex :type Integer) (bFromSweep :type Boolean) (SweepResult :type Hit%20Result%20Structure%20%28by%20ref%29))
  (if (Variables|Default|GethasDelivery)
    (bind _asbp_first_person_character (Utilities|Casting|CastToBP_FirstPersonCharacter OtherActor))
    (Default|DropOff _asbp_first_person_character (Variables|Default|GetDelivery%20Count))
    (Variables|Default|SetDelivery%20Count 0)
    (Variables|Default|SethasDelivery false)
    (Rendering|SetVisibility (Variables|Default|GetWaypoint) false false)))

(event Custom|Delivery
  (Rendering|SetVisibility (Variables|Default|GetWaypoint) true false)
  (Variables|Default|SethasDelivery true)
  (Math|Integer|IncrementInt (Variables|Default|GetDelivery%20Count)))

(fn ConstructionScript)